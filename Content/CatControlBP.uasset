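; Player-controlled cat for a top-down, music-synced shooter, moving on input axes and rotating toward the cursor.
; Tick re-arms shooting at each GlobalMusic half-beat, limiting either attack to one bullet per beat; the two attacks differ only in material.
; Overlapping damaging hostile projectiles reduces health, updates the heart widget and grants invincibility lasting four beats.
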(event Collision|EventActorBeginOverlap
  (params (OtherActor :type Actor%20Object%20Reference))
  (bind _asprojectile_base_bp (Utilities|Casting|CastToProjectileBaseBP OtherActor))
  (if (not (> (Variables|Default|GetInvincibility%20Time) 0.0))
    (if (and (not (Variables|/Game/Projectiles/ProjectileBaseBP.ProjectileBaseBP_C|GetFriendly _asprojectile_base_bp)) (Default|IsDamaging _asprojectile_base_bp))
      (CallFunction|TakeDamage (Default|GetDamage _asprojectile_base_bp))
      (if (Default|IsDestroyedonHit _asprojectile_base_bp)
        (Actor|DestroyActor _asprojectile_base_bp)))))

(event EventBeginPlay
  (bind _returnvalue (Actor|GetActorOfClass "/Game/GlobalMusic.GlobalMusic_C"))
  (Variables|Default|SetGlobal%20Music _returnvalue))

(event EventTick
  (params (DeltaSeconds :type Float%20%28single-precision%29))
  (bind _global_music (Variables|Default|GetGlobal%20Music))
  (Transformation|SetActorRotation (Math|Rotator|FindLookatRotation (* (Transformation|GetActorLocation) "1.000000,1.000000,0.000000") (* (.Location (Collision|BreakHitResult (.HitResult (Game|Player|GetHitResultUnderCursorbyChannel (Game|GetPlayerController 0) "TraceTypeQuery1" true)))) "1.000000,1.000000,0.000000")))
  (Transformation|SetActorLocation (+ (Transformation|GetActorLocation) (* (* (Math|Vector|Normalize (Math|Vector|MakeVector (Input|AxisValues|GetPlayerSide) (Input|AxisValues|GetPlayerUp) 0.0)) DeltaSeconds) (Variables|Default|GetMovement%20Speed))) false false)
  (Variables|Default|SetInvincibility%20Time (- (Variables|Default|GetInvincibility%20Time) DeltaSeconds))
  (if (and (< (Variables|/Game/GlobalMusic.GlobalMusic_C|GetPrev%20Beat%20Fraction _global_music) 0.5) (>= (Variables|/Game/GlobalMusic.GlobalMusic_C|GetBeat%20Fraction _global_music) 0.5))
    (Variables|Default|SetCan%20Shoot true)))

(event Input|ActionEvents|InputActionAttack1
  (params (Key :type Key%20Structure :default "None"))
  (:Pressed
    (CallFunction|FireBullet false)))

(event Input|ActionEvents|InputActionAttack2
  (params (Key :type Key%20Structure :default "None"))
  (:Pressed
    (CallFunction|FireBullet true)))

(fn ConstructionScript)

(fn TakeDamage
  (params (Damage :type Integer))
  (CallFunction|AddHealth (- 0 Damage))
  (Variables|Default|SetInvincibility%20Time (* (Default|GetSecondsPerBeat (Variables|Default|GetGlobal%20Music)) 4.0)))

(fn AddHealth
  (params (Added%20Health :type Integer))
  (bind _output_get (Variables|Default|SetHealth (+ (Variables|Default|GetHealth) Added%20Health)))
  (bind _foundwidgets (Widget|GetAllWidgetsOfClass "/Game/PlayerHealthDisplay.PlayerHealthDisplay_C" true))
  (Default|SetHeartImages (Utilities|Array|Get(acopy) _foundwidgets) _output_get))

(fn FireBullet
  (params (Attack%202 :type Boolean))
  (bind _returnvalue (Transformation|GetActorTransform))
  (bind (_location _rotation) (Math|Transform|BreakTransform _returnvalue))
  (if (Variables|Default|GetCan%20Shoot)
    (Variables|Default|SetCan%20Shoot false)
    (bind _returnvalue_2 (Game|SpawnActorfromClass "/Game/Projectiles/Bullet.Bullet_C" (Math|Transform|MakeTransform _location _rotation (Math|Conversions|ToVector(Float) (Math|Float|MakeLiteralFloat 0.7))) "AlwaysSpawn" 0 self))
    (Variables|/Game/Projectiles/Bullet.Bullet_C|SetDoes%20Pulse%20Movement _returnvalue_2 false)
    (Default|SetSpeed _returnvalue_2 2e+02)
    (Variables|/Game/Projectiles/ProjectileBaseBP.ProjectileBaseBP_C|SetDamage _returnvalue_2 5)
    (Default|SetMaterial _returnvalue_2 (select Attack%202 "/Game/Projectiles/PlayerBulletMaterial2.PlayerBulletMaterial2" "/Game/Projectiles/PlayerBulletMaterial1.PlayerBulletMaterial1"))
    (Audio|PlaySound2D "/Game/Assets/Audio/Sounds/hit_test.hit_test" 1.0 1.0 0.0 0 0)))