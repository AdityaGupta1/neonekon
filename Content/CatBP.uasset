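; CatBP is a player-controlled cat actor with basic movement and mouse turning.
; PlayerForward and PlayerSide axis inputs offset its location along its forward and right vectors at a fixed per-frame step, without sweep or delta-time scaling.
; Tick rotates the forward vector around world Z by the first player controller's horizontal mouse delta, then rebuilds the actor rotation from that vector.
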(event EventBeginPlay)

(event Collision|EventActorBeginOverlap
  (params (OtherActor :type Actor%20Object%20Reference)))

(event EventTick
  (params (DeltaSeconds :type Float%20%28single-precision%29))
  (Transformation|SetActorRotation (Math|Rotator|MakeRotfromX (Math|Vector|RotateVectorAroundAxis (Math|Rotator|GetRotationXVector (Transformation|GetActorRotation)) (.DeltaX (Class|PlayerController|GetInputMouseDelta (Game|GetPlayerController 0))) "0.000000,0.000000,1.000000"))))

(event Input|AxisEvents|InputAxisPlayerForward
  (params (AxisValue :type Float%20%28single-precision%29))
  (Transformation|SetActorLocation (+ (* (* AxisValue 3.0) (Math|Rotator|GetRotationXVector (Transformation|GetActorRotation))) (Transformation|GetActorLocation)) false false))

(event Input|AxisEvents|InputAxisPlayerSide
  (params (AxisValue :type Float%20%28single-precision%29))
  (Transformation|SetActorLocation (+ (* (* AxisValue 3.0) (Math|Vector|GetRightVector (Transformation|GetActorRotation))) (Transformation|GetActorLocation)) false false))

(fn ConstructionScript)