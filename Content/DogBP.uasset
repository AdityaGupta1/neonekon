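; DogBP is a dog enemy that runs beat-driven attack phases.
; On BeginPlay it builds an AttackPhaseManager, loads the "dog 1" phases for itself and fills its health.
; ActionOnBeat forwards each beat to that manager; a random position jitter there is disabled.
; AddHealth adjusts health without clamping and updates the first EnemyHealthDisplay widget found with the health ratio.
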(event Custom|ActionOnBeat
  (Transformation|SetActorLocation (+ (Transformation|GetActorLocation) (Math|Vector|MakeVector (Math|Conversions|ToFloat(Integer) (* (Math|Random|RandomIntegerinRange -1 1) 10)) (Math|Conversions|ToFloat(Integer) (* (Math|Random|RandomIntegerinRange -1 1) 10)) 0.0)) false false)
  (Class|AttackPhaseManager|OnBeat (Variables|Default|GetAttack%20Phase%20Manager) self))

(event EventBeginPlay
  (bind _returnvalue (Game|ConstructObjectfromClass "/Script/neonekon.AttackPhaseManager"))
  (bind _output_get (Variables|Default|SetAttack%20Phase%20Manager _returnvalue))
  (Class|AttackPhaseManager|LoadPhases _output_get "dog 1" self)
  (bind _output_get_2 (Variables|Default|SetMax%20Health 1000))
  (Variables|Default|SetHealth _output_get_2))

(fn ConstructionScript)

(fn AddHealth
  (params (Added%20Health :type Integer))
  (Variables|Default|SetHealth (+ (Variables|Default|GetHealth) Added%20Health))
  (bind _foundwidgets (Widget|GetAllWidgetsOfClass "/Game/EnemyHealthDisplay.EnemyHealthDisplay_C" true))
  (Default|SetBarPercentage (Utilities|Array|Get(acopy) _foundwidgets) (/ (Math|Conversions|ToFloat(Integer) (Variables|Default|GetHealth)) (Variables|Default|GetMax%20Health))))