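; Base projectile Blueprint that carries damage settings and a lifespan measured in musical beats.
; On BeginPlay it caches the GlobalMusic actor, whose seconds-per-beat multiplied by DurationBeats gives the lifespan in seconds.
; SetLifespanFromBeats applies that value but is not called within this Blueprint.
; Getters expose damage, whether it damages and whether it is destroyed on hit, while SetMaterial is an empty stub.
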(event EventBeginPlay
  (bind _returnvalue (Actor|GetActorOfClass "/Game/GlobalMusic.GlobalMusic_C"))
  (Variables|Default|SetGlobal%20Music _returnvalue))

(fn ConstructionScript)

(fn SetLifespanfromBeats
  (Actor|SetLifeSpan (CallFunction|ConvertLifespanfromBeats)))

(fn ConvertLifespanfromBeats
  (return (* (Default|GetSecondsPerBeat (Variables|Default|GetGlobal%20Music)) (Variables|Default|GetdurationBeats))))

(fn IsDamaging
  (return (Variables|Default|GetDamaging)))

(fn IsDestroyedonHit
  (return (Variables|Default|GetDestroyed%20on%20Hit)))

(fn GetDamage
  (return (Variables|Default|GetDamage)))

(fn SetMaterial
  (params (Material :type Material%20Instance%20Object%20Reference)))